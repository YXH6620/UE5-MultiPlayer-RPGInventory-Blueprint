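; BP_Player is the player pawn for FogTown, handling movement and horizontal look through Enhanced Input.
; On BeginPlay it casts its controller to PC_FogTown and, if that succeeds, adds the IMC_Default mapping context.
; IA_Movement drives movement along the actor's forward (X) and right (Y) vectors.
; IA_Look feeds controller yaw only, with no pitch input.
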(event `self.ReceiveBeginPlay`
  (bind _aspc_fog_town (cast `/Game/Blueprints/PC_FogTown` (`self.GetController`)))
  (`EnhancedInputSubsystemInterface.AddMappingContext` (pcsubsystem `EnhancedInputLocalPlayerSubsystem` _aspc_fog_town) "/Game/Blueprints/Player/IMC_Default.IMC_Default" 0 (struct)))

(event `EnhancedInput|/Game/Blueprints/Player/IA_Movement`
  (params (ActionValue :type "Vector2D Structure") (ElapsedSeconds :type "Float (double-precision)") (TriggeredSeconds :type "Float (double-precision)") (InputAction :type "InputAction Object Reference" :default "/Game/Blueprints/Player/IA_Movement.IA_Movement"))
  (:`Triggered`
    (`self.AddMovementInput` (`self.GetActorForwardVector`) ActionValue_X)
    (`self.AddMovementInput` (`self.GetActorRightVector`) ActionValue_Y)))

(event `EnhancedInput|/Game/Blueprints/Player/IA_Look`
  (params (ActionValue :type "Float (double-precision)") (ElapsedSeconds :type "Float (double-precision)") (TriggeredSeconds :type "Float (double-precision)") (InputAction :type "InputAction Object Reference" :default "/Game/Blueprints/Player/IA_Look.IA_Look"))
  (:`Triggered`
    (`self.AddControllerYawInput` ActionValue)))

(fn `UserConstructionScript`)