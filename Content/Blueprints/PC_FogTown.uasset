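; FogTown player controller that creates the main WBP_Main UI on BeginPlay and shows or hides it as the inventory.
; An Open/Close event forwards a widget type and open flag to a client event, which branches to OpenWidget or CloseWidget.
; Only Inventory is handled, toggling viewport presence and IsOpenInventory.
; OpenWidget does not store a newly created widget in MainUI, which CloseWidget removes.
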(event `self.ReceiveBeginPlay`
  (`self.Initialize Widget`))

(event `Initialize Widget`
  (bind _returnvalue (`|CreateWidget` "/Game/UI/WBP_Main.WBP_Main_C"))
  (bind _output_get (set `self.MainUI` _returnvalue))
  (`UserWidget.AddToViewport` _output_get 0))

(event `Open/Close Widget`
  (params (Widget :type "/Game/Blueprints/Enum/E_GameWidget Enum" :default "NewEnumerator0") (Open :type Boolean))
  (`self.Client_Open/Close Widget` Widget Open))

(event `Client_Open/Close Widget`
  (params (Widget :type "/Game/Blueprints/Enum/E_GameWidget Enum" :default "NewEnumerator0") (Open :type Boolean))
  (if Open
    (`self.Open Widget` Widget)
    (else
      (`self.Close Widget` Widget))))

(fn `Close Widget`
  (params (widget :type "/Game/Blueprints/Enum/E_GameWidget Enum" :default "NewEnumerator0"))
  (switch `/Game/Blueprints/Enum/E_GameWidget` widget
    (:`NewEnumerator0`
      (bind _mainui (`self.MainUI`)
        (:`then`
          (`Widget.RemoveFromParent` _mainui)
          (set `self.Is Open Inventory` false))
        (:`else`)))))

(fn `GetPlayerControllerRef`
  (returns (`Fog Town Controller` :type "/Game/Blueprints/PC_FogTown Object Reference"))
  (return self))

(fn `Open Widget`
  (params (widget :type "/Game/Blueprints/Enum/E_GameWidget Enum" :default "NewEnumerator0"))
  (switch `/Game/Blueprints/Enum/E_GameWidget` widget
    (:`NewEnumerator0`
      (`self.MainUI`
        (:`then`
          _)
        (:`else`
          (bind _returnvalue (`|CreateWidget` "/Game/UI/WBP_Main.WBP_Main_C"))))
      (`UserWidget.AddToViewport` _returnvalue 0)
      (set `self.Is Open Inventory` true))))

(fn `UserConstructionScript`)